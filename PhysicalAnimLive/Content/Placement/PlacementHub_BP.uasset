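; Clickable tower build spot for a tower defense game that lets the player buy a tower in its place.
; Clicking the mesh opens a placement widget, guarded against duplicates, with buttons for double-barrel, slow, homing and gas towers plus Close.
; Each purchase checks TDF_Gamemode points, spawns the tower, deducts points and destroys the hub, or plays an insufficient-funds sound.
; The gas tower's affordability check is lower than the amount it deducts.
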(event OnClicked(StaticMesh)
  (params (TouchedComponent :type Primitive%20Component%20Object%20Reference) (ButtonPressed :type Key%20Structure))
  (if (not (Variables|Default|GetIsAlreadyActive))
    (Variables|Default|SetIsAlreadyActive true)
    (bind _returnvalue (UserInterface|CreateWidget "/Game/UI/Placement_UI.Placement_UI_C" (Game|GetPlayerController 0)))
    (UserInterface|Viewport|AddtoViewport _returnvalue 0)
    (EventDispatchers|AssignOnClicked (Variables|/Game/UI/Placement_UI.Placement_UI_C|Get2BTower_BTN _returnvalue) (delegate Custom|OnClicked4BTower_BTN))
    (EventDispatchers|AssignOnClicked (Variables|/Game/UI/Placement_UI.Placement_UI_C|GetBTower_BTN _returnvalue) (delegate Custom|OnClickedBTower_BTN))
    (EventDispatchers|AssignOnClicked (Variables|/Game/UI/Placement_UI.Placement_UI_C|GetHomingTower_BTN _returnvalue) (delegate Custom|OnClicked_Event_0))
    (EventDispatchers|BindEventtoOnClicked (Variables|/Game/UI/Placement_UI.Placement_UI_C|GetAcid_BTN _returnvalue) (delegate Custom|Acid_ClickedON))
    (EventDispatchers|BindEventtoOnClicked (Variables|/Game/UI/Placement_UI.Placement_UI_C|GetClose_BTN _returnvalue) (delegate Custom|Exit))))

(event Custom|OnClicked_Event_0
  (bind _returnvalue (Transformation|GetActorLocation))
  (bind _astdf_gamemode (Utilities|Casting|CastToTDF_Gamemode (Game|GetGameMode)))
  (if (>= (Variables|/Game/User/TDF_Gamemode.TDF_Gamemode_C|GetPoints _astdf_gamemode) 500)
    (Audio|PlaySoundatLocation "/Game/Audio/BuySound.BuySound" _returnvalue "0, 0, 0" 1.0 1.0 0.0 0 0 0)
    (Game|SpawnActorfromClass "/Game/Towers/HomingTower/HomingTower_BP.HomingTower_BP_C" (Transformation|GetActorTransform) "Undefined" 0 0)
    (Variables|/Game/User/TDF_Gamemode.TDF_Gamemode_C|SetPoints _astdf_gamemode (- (Variables|/Game/User/TDF_Gamemode.TDF_Gamemode_C|GetPoints _astdf_gamemode) 500))
    (Widget|RemovefromParent (stale OnClicked(StaticMesh) _returnvalue))
    (Actor|DestroyActor)
    (Variables|Default|SetIsAlreadyActive false)
    (else
      (Audio|PlaySoundatLocation "/Game/Audio/InsuffecientFunds.InsuffecientFunds" _returnvalue "0, 0, 0" 0.7 1.0 0.0 0 0 0))))

(event Custom|OnClicked4BTower_BTN
  (bind _returnvalue (Transformation|GetActorLocation))
  (bind _astdf_gamemode (Utilities|Casting|CastToTDF_Gamemode (Game|GetGameMode)))
  (if (>= (Variables|/Game/User/TDF_Gamemode.TDF_Gamemode_C|GetPoints _astdf_gamemode) 350)
    (Audio|PlaySoundatLocation "/Game/Audio/BuySound.BuySound" _returnvalue "0, 0, 0" 1.0 1.0 0.0 0 0 0)
    (Game|SpawnActorfromClass "/Game/Towers/2BarrelTower/2BarrelTowerBp.2BarrelTowerBp_C" (Transformation|GetActorTransform) "Undefined" 0 0)
    (Variables|/Game/User/TDF_Gamemode.TDF_Gamemode_C|SetPoints _astdf_gamemode (- (Variables|/Game/User/TDF_Gamemode.TDF_Gamemode_C|GetPoints _astdf_gamemode) 350))
    (Widget|RemovefromParent (stale OnClicked(StaticMesh) _returnvalue))
    (Actor|DestroyActor)
    (Variables|Default|SetIsAlreadyActive false)
    (else
      (Audio|PlaySoundatLocation "/Game/Audio/InsuffecientFunds.InsuffecientFunds" _returnvalue "0, 0, 0" 0.7 1.0 0.0 0 0 0))))

(event Custom|OnClickedBTower_BTN
  (bind _returnvalue (Transformation|GetActorLocation))
  (bind _astdf_gamemode (Utilities|Casting|CastToTDF_Gamemode (Game|GetGameMode)))
  (if (>= (Variables|/Game/User/TDF_Gamemode.TDF_Gamemode_C|GetPoints _astdf_gamemode) 400)
    (Audio|PlaySoundatLocation "/Game/Audio/BuySound.BuySound" _returnvalue "0, 0, 0" 1.0 1.0 0.0 0 0 0)
    (Game|SpawnActorfromClass "/Game/Towers/SlowTower/SlowTower_BP.SlowTower_BP_C" (Transformation|GetActorTransform) "Undefined" 0 0)
    (Variables|/Game/User/TDF_Gamemode.TDF_Gamemode_C|SetPoints _astdf_gamemode (- (Variables|/Game/User/TDF_Gamemode.TDF_Gamemode_C|GetPoints _astdf_gamemode) 400))
    (Widget|RemovefromParent (stale OnClicked(StaticMesh) _returnvalue))
    (Actor|DestroyActor)
    (Variables|Default|SetIsAlreadyActive false)
    (else
      (Audio|PlaySoundatLocation "/Game/Audio/InsuffecientFunds.InsuffecientFunds" _returnvalue "0, 0, 0" 0.7 1.0 0.0 0 0 0))))

(event Custom|Acid_ClickedON
  (bind _returnvalue (Transformation|GetActorLocation))
  (bind _astdf_gamemode (Utilities|Casting|CastToTDF_Gamemode (Game|GetGameMode)))
  (if (>= (Variables|/Game/User/TDF_Gamemode.TDF_Gamemode_C|GetPoints _astdf_gamemode) 350)
    (Audio|PlaySoundatLocation "/Game/Audio/BuySound.BuySound" _returnvalue "0, 0, 0" 1.0 1.0 0.0 0 0 0)
    (Game|SpawnActorfromClass "/Game/Towers/GasTower/GasTower_BP.GasTower_BP_C" (Transformation|GetActorTransform) "Undefined" 0 0)
    (Variables|/Game/User/TDF_Gamemode.TDF_Gamemode_C|SetPoints _astdf_gamemode (- (Variables|/Game/User/TDF_Gamemode.TDF_Gamemode_C|GetPoints _astdf_gamemode) 700))
    (Widget|RemovefromParent (stale OnClicked(StaticMesh) _returnvalue))
    (Actor|DestroyActor)
    (Variables|Default|SetIsAlreadyActive false)
    (else
      (Audio|PlaySoundatLocation "/Game/Audio/InsuffecientFunds.InsuffecientFunds" _returnvalue "0, 0, 0" 0.7 1.0 0.0 0 0 0))))

(event Custom|Exit
  (Widget|RemovefromParent (stale OnClicked(StaticMesh) _returnvalue))
  (Variables|Default|SetIsAlreadyActive false))

(event EventBeginPlay)

(event Collision|EventActorBeginOverlap
  (params (OtherActor :type Actor%20Object%20Reference)))

(event EventTick
  (params (DeltaSeconds :type Float%20%28single-precision%29)))

(fn ConstructionScript)