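; Base enemy Blueprint that walks to the core and takes damage-over-time and slow effects.
; On BeginPlay it ignores collision with fellow enemies, caches the spawner and moves toward the first Core_BP found.
; Looping timers drive acid and long-burn damage, halved when Invigored, while SlowCharacter temporarily cuts walk speed.
; Tick polls health, and on death decrements the spawner's count, destroys the enemy and shows LevelFinish_UI when none remain.
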(event Custom|Slow%20Character
  (Variables|/Script/Engine.CharacterMovementComponent|SetMaxWalkSpeed (Variables|Character|GetCharacterMovement) 5e+01)
  (Utilities|FlowControl|Delay 2.0)
  (Variables|/Script/Engine.CharacterMovementComponent|SetMaxWalkSpeed (Variables|Character|GetCharacterMovement) (Variables|Default|GetDefaultWalkSpeed)))

(event Custom|Damage%20over%20Time
  (bind _returnvalue (Utilities|Time|SetTimerbyFunctionName 0 "Acid Damage" 0.75 true)))

(event Custom|Stop%20Damage%20over%20time
  (Utilities|Time|ClearandInvalidateTimerbyHandle (stale Custom|Damage%20over%20Time _returnvalue)))

(event Custom|StartLongDamage
  (bind _returnvalue (Utilities|Time|SetTimerbyFunctionName 0 "LongBurn Damage" 0.75 true)))

(event Custom|StopLongDamage
  (Utilities|Time|ClearandInvalidateTimerbyHandle (stale Custom|StartLongDamage _returnvalue)))

(event Custom|LongBurn%20Damage
  (if (Variables|Default|GetInvigored)
    (Variables|Default|SetHealth (- (Variables|Default|GetHealth) 1e+01))
    (else
      (Variables|Default|SetHealth (- (Variables|Default|GetHealth) 2e+01)))))

(event Custom|Acid%20Damage
  (if (Variables|Default|GetInvigored)
    (Variables|Default|SetHealth (- (Variables|Default|GetHealth) 5.0))
    (else
      (Variables|Default|SetHealth (- (Variables|Default|GetHealth) 1e+01)))))

(event EventBeginPlay
  (Variables|Default|SetDefaultWalkSpeed (Variables|/Script/Engine.CharacterMovementComponent|GetMaxWalkSpeed (Variables|Character|GetCharacterMovement)))
  (bind _outactors (Actor|GetAllActorsOfClass "BaseEnemyClass_BP_C"))
  (for _array_element _outactors
    (Collision|IgnoreActorwhenMoving (Variables|Collision|GetCapsuleComponent) _array_element true)
    (bind _outactors_2 (Actor|GetAllActorsOfClass "/Game/AI/EnemySpawner.EnemySpawner_C"))
    (Variables|Default|SetSpawner (Utilities|Array|Get(acopy) _outactors_2))
    (bind _outactors_3 (Actor|GetAllActorsOfClass "/Game/Core/Core_BP.Core_BP_C"))
    (Variables|Default|SetPatrolPoints _outactors_3)
    (AI|Navigation|SimpleMovetoActor (Pawn|GetController) (Utilities|Array|Get(acopy) (Variables|Default|GetPatrolPoints)))))

(event EventTick
  (params (DeltaSeconds :type Float%20%28single-precision%29))
  (if (<= (Variables|Default|GetHealth) 0.0)
    (bind _asenemy_spawner (Utilities|Casting|CastToEnemySpawner (Variables|Default|GetSpawner)))
    (Variables|/Game/AI/EnemySpawner.EnemySpawner_C|SetSpawnAmount _asenemy_spawner (- (Variables|/Game/AI/EnemySpawner.EnemySpawner_C|GetSpawnAmount _asenemy_spawner) 1))
    (Actor|DestroyActor)
    (bind _outactors (Actor|GetAllActorsOfClass "/Game/AI/EnemySpawner.EnemySpawner_C"))
    (if (<= (Variables|/Game/AI/EnemySpawner.EnemySpawner_C|GetSpawnAmount (Utilities|Array|Get(acopy) _outactors)) 0)
      (Game|GetCurrentLevelName true)
      (bind _returnvalue (UserInterface|CreateWidget "/Game/UI/LevelFinish_UI.LevelFinish_UI_C" (Game|GetPlayerController 0)))
      (UserInterface|Viewport|AddtoViewport _returnvalue 0))))

(fn ConstructionScript)