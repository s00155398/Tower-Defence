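; Invigorator enemy that buffs nearby enemies by flagging them as invigored.
; Its InvigorationRange overlap events match actors against the TDF_Gamemode EnemyTags list, setting Invigored on BaseEnemyClass_BP actors on entry and clearing it on exit.
; The flag is a plain boolean, so leaving one range clears it even inside another.
; Tick runs parent logic, then adds points to the game mode on every frame Health is at or below zero, with no one-time guard.
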(event OnComponentBeginOverlap(InvigorationRange)
  (params (OverlappedComponent :type Primitive%20Component%20Object%20Reference) (OtherActor :type Actor%20Object%20Reference) (OtherComp :type Primitive%20Component%20Object%20Reference) (OtherBodyIndex :type Integer) (bFromSweep :type Boolean) (SweepResult :type Hit%20Result%20Structure%20%28by%20ref%29))
  (bind _astdf_gamemode (Utilities|Casting|CastToTDF_Gamemode (Game|GetGameMode)))
  (for _array_element (Variables|/Game/User/TDF_Gamemode.TDF_Gamemode_C|GetEnemyTags _astdf_gamemode)
    (if (Actor|ActorHasTag OtherActor _array_element)
      (bind _asbase_enemy_class_bp (Utilities|Casting|CastToBaseEnemyClass_BP OtherActor))
      (Variables|/Game/AI/Enemies/BaseEnemyClass_BP.BaseEnemyClass_BP_C|SetInvigored _asbase_enemy_class_bp true))))

(event OnComponentEndOverlap(InvigorationRange)
  (params (OverlappedComponent :type Primitive%20Component%20Object%20Reference) (OtherActor :type Actor%20Object%20Reference) (OtherComp :type Primitive%20Component%20Object%20Reference) (OtherBodyIndex :type Integer))
  (bind _astdf_gamemode (Utilities|Casting|CastToTDF_Gamemode (Game|GetGameMode)))
  (for _array_element (Variables|/Game/User/TDF_Gamemode.TDF_Gamemode_C|GetEnemyTags _astdf_gamemode)
    (if (Actor|ActorHasTag OtherActor _array_element)
      (bind _asbase_enemy_class_bp (Utilities|Casting|CastToBaseEnemyClass_BP OtherActor))
      (Variables|/Game/AI/Enemies/BaseEnemyClass_BP.BaseEnemyClass_BP_C|SetInvigored _asbase_enemy_class_bp false))))

(event EventBeginPlay
  (|CallParentFunction) ; This node is disabled and will not be called.\nDrag off pins to build functionality.
)

(event Collision|EventActorBeginOverlap
  (params (OtherActor :type Actor%20Object%20Reference)))

(event EventTick
  (params (DeltaSeconds :type Float%20%28single-precision%29))
  (|CallParentFunction DeltaSeconds)
  (if (<= (Variables|Default|GetHealth) 0.0)
    (bind _astdf_gamemode (Utilities|Casting|CastToTDF_Gamemode (Game|GetGameMode)))
    (Variables|/Game/User/TDF_Gamemode.TDF_Gamemode_C|SetPoints _astdf_gamemode (+ (Variables|/Game/User/TDF_Gamemode.TDF_Gamemode_C|GetPoints _astdf_gamemode) 100))))

(fn ConstructionScript
  (|CallParentFunction))