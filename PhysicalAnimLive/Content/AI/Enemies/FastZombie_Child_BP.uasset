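; Fast zombie enemy child Blueprint that adds a score reward for its death on top of inherited parent behavior.
; Each Tick runs the parent Tick, then checks Health and, at zero or below, adds 200 to Points on TDF_Gamemode.
; This graph has no once-only guard, so points repeat every frame the actor keeps ticking at zero health.
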(event EventBeginPlay
  (|CallParentFunction) ; This node is disabled and will not be called.\nDrag off pins to build functionality.
)

(event Collision|EventActorBeginOverlap
  (params (OtherActor :type Actor%20Object%20Reference)))

(event EventTick
  (params (DeltaSeconds :type Float%20%28single-precision%29))
  (|CallParentFunction DeltaSeconds)
  (if (<= (Variables|Default|GetHealth) 0.0)
    (bind _astdf_gamemode (Utilities|Casting|CastToTDF_Gamemode (Game|GetGameMode)))
    (Variables|/Game/User/TDF_Gamemode.TDF_Gamemode_C|SetPoints _astdf_gamemode (+ (Variables|/Game/User/TDF_Gamemode.TDF_Gamemode_C|GetPoints _astdf_gamemode) 200))))

(fn ConstructionScript
  (|CallParentFunction))