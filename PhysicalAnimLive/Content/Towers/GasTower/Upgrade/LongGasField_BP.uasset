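; LongGasField_BP is a short-lived gas hazard, part of the Gas Tower upgrade, that deals long damage to enemies inside it.
; Box overlaps match actors against the game mode's EnemyTags, then call StartLongDamage on entry and StopLongDamage on exit on BaseEnemyClass_BP, which owns the damage logic.
; On BeginPlay it plays an attached hiss sound and destroys itself after about three seconds.
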(event OnComponentBeginOverlap(Box)
  (params (OverlappedComponent :type Primitive%20Component%20Object%20Reference) (OtherActor :type Actor%20Object%20Reference) (OtherComp :type Primitive%20Component%20Object%20Reference) (OtherBodyIndex :type Integer) (bFromSweep :type Boolean) (SweepResult :type Hit%20Result%20Structure%20%28by%20ref%29))
  (bind _astdf_gamemode (Utilities|Casting|CastToTDF_Gamemode (Game|GetGameMode)))
  (for _array_element (Variables|/Game/User/TDF_Gamemode.TDF_Gamemode_C|GetEnemyTags _astdf_gamemode)
    (if (Actor|ActorHasTag OtherActor _array_element)
      (bind _asbase_enemy_class_bp (Utilities|Casting|CastToBaseEnemyClass_BP OtherActor))
      (Default|StartLongDamage _asbase_enemy_class_bp))))

(event OnComponentEndOverlap(Box)
  (params (OverlappedComponent :type Primitive%20Component%20Object%20Reference) (OtherActor :type Actor%20Object%20Reference) (OtherComp :type Primitive%20Component%20Object%20Reference) (OtherBodyIndex :type Integer))
  (bind _astdf_gamemode (Utilities|Casting|CastToTDF_Gamemode (Game|GetGameMode)))
  (for _array_element (Variables|/Game/User/TDF_Gamemode.TDF_Gamemode_C|GetEnemyTags _astdf_gamemode)
    (if (Actor|ActorHasTag OtherActor _array_element)
      (bind _asbase_enemy_class_bp (Utilities|Casting|CastToBaseEnemyClass_BP OtherActor))
      (Default|StopLongDamage _asbase_enemy_class_bp))))

(event EventBeginPlay
  (Audio|SpawnSoundAttached "/Game/Audio/Hiss.Hiss" (Variables|Default|GetBox) "None" "0, 0, 0" "0, 0, 0" "KeepRelativeOffset" false 1.0 2.0 0.0 0 0)
  (Utilities|FlowControl|Delay 3.1)
  (Actor|DestroyActor))

(event Collision|EventActorBeginOverlap
  (params (OtherActor :type Actor%20Object%20Reference)))

(fn ConstructionScript)