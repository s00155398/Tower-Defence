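; Projectile for the upgraded gas tower that bursts into a long gas field when it hits an enemy.
; On overlap, it checks the other actor against the gamemode's enemy tags, then spawns an explosion effect, a sound and a LongGasField_BP at that actor's location and destroys itself.
; A round that hits no enemy destroys itself after a short delay from BeginPlay.
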(event OnComponentBeginOverlap(CollisionComponent)
  (params (OverlappedComponent :type Primitive%20Component%20Object%20Reference) (OtherActor :type Actor%20Object%20Reference) (OtherComp :type Primitive%20Component%20Object%20Reference) (OtherBodyIndex :type Integer) (bFromSweep :type Boolean) (SweepResult :type Hit%20Result%20Structure%20%28by%20ref%29))
  (bind _returnvalue (Transformation|GetActorLocation OtherActor))
  (bind _astdf_gamemode (Utilities|Casting|CastToTDF_Gamemode (Game|GetGameMode)))
  (for _array_element (Variables|/Game/User/TDF_Gamemode.TDF_Gamemode_C|GetEnemyTags _astdf_gamemode)
    (if (Actor|ActorHasTag OtherActor _array_element)
      (Effects|SpawnEmitteratLocation "/Game/Materials/Effects/P_GasExplosion.P_GasExplosion" _returnvalue)
      (Audio|SpawnSoundatLocation "/Game/Audio/AcidBreak.AcidBreak" _returnvalue "0, 0, 0" 0.15 1.0 2.0 0 0)
      (Game|SpawnActorfromClass "/Game/Towers/GasTower/Upgrade/LongGasField_BP.LongGasField_BP_C" (Math|Conversions|ToTransform(Vector) _returnvalue) "Undefined" 0 0)
      (Actor|DestroyActor))))

(event EventBeginPlay
  (Utilities|FlowControl|Delay 5.0)
  (Actor|DestroyActor))

(fn ConstructionScript)