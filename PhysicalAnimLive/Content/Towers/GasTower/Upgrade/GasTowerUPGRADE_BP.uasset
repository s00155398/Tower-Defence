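; Upgraded gas tower for a tower defense game that automatically fires gas rounds at tagged enemies inside its FireField.
; Overlap events maintain the target list, and a polled delay loop yaws the head toward the first entry.
; The first target starts a self-repeating fire loop that spawns projectiles with sound and muzzle effects.
; Clicking the tower opens a revert widget that can replace it with a placement hub and refund points.
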(event OnComponentBeginOverlap(FireField)
  (params (OverlappedComponent :type Primitive%20Component%20Object%20Reference) (OtherActor :type Actor%20Object%20Reference) (OtherComp :type Primitive%20Component%20Object%20Reference) (OtherBodyIndex :type Integer) (bFromSweep :type Boolean) (SweepResult :type Hit%20Result%20Structure%20%28by%20ref%29))
  ;[1 1 1] Track Targets that enter the firing triggerbox
  (bind _aspawn (Utilities|Casting|CastToPawn OtherActor))
  (bind _astdf_gamemode (Utilities|Casting|CastToTDF_Gamemode (Game|GetGameMode)))
  (for _array_element (Variables|/Game/User/TDF_Gamemode.TDF_Gamemode_C|GetEnemyTags _astdf_gamemode)
    (if (Actor|ActorHasTag _aspawn _array_element)
      (Utilities|Array|Add (Variables|Default|GetEnemyTargets) OtherActor))))

(event OnClicked(TriggerBox)
  (params (TouchedComponent :type Primitive%20Component%20Object%20Reference) (ButtonPressed :type Key%20Structure))
  (if (not (Variables|Default|GetUIActive))
    (Variables|Default|SetUIActive true)
    (bind _returnvalue (UserInterface|CreateWidget "/Game/UI/Revert_UI.Revert_UI_C" (Game|GetPlayerController 0)))
    (UserInterface|Viewport|AddtoViewport _returnvalue 0)
    (EventDispatchers|AssignOnClicked (Variables|/Game/UI/Revert_UI.Revert_UI_C|GetClose_BTN _returnvalue) (delegate Custom|Close_Click))
    (EventDispatchers|BindEventtoOnClicked (Variables|/Game/UI/Revert_UI.Revert_UI_C|GetRevert_BTN _returnvalue) (delegate Custom|Revert_Click))))

(event OnComponentEndOverlap(FireField)
  (params (OverlappedComponent :type Primitive%20Component%20Object%20Reference) (OtherActor :type Actor%20Object%20Reference) (OtherComp :type Primitive%20Component%20Object%20Reference) (OtherBodyIndex :type Integer))
  ;[1 1 1] Track Targets that enter the firing triggerbox
  (bind _aspawn (Utilities|Casting|CastToPawn OtherActor))
  (bind _astdf_gamemode (Utilities|Casting|CastToTDF_Gamemode (Game|GetGameMode)))
  (for _array_element (Variables|/Game/User/TDF_Gamemode.TDF_Gamemode_C|GetEnemyTags _astdf_gamemode)
    (if (Actor|ActorHasTag _aspawn _array_element)
      (Utilities|Array|RemoveItem (Variables|Default|GetEnemyTargets) OtherActor))))

(event Custom|AutoFire
  (bind _towerhead (Variables|Default|GetTowerHead))
  (bind _returnvalue (Transformation|GetWorldRotation _towerhead))
  (bind _returnvalue_2 (Math|Rotator|GetRotationXVector _returnvalue))
  (bind _returnvalue_3 (Math|Vector|Normalize _returnvalue_2))
  (bind _returnvalue_4 (* _returnvalue_3 1.0))
  ;[1 1 1] Auto Firing Loop
  (Utilities|FlowControl|Delay 3.0 :!label _label)
  (if (Variables|Default|GetAutoShoot)
    (Variables|Default|SetShootDirection _returnvalue_4)
    (Variables|Default|SetSpawnLocation (+ _returnvalue_4 (Transformation|GetWorldLocation _towerhead)))
    (Utilities|FlowControl|DoOnce false :!label _label_2
      (:Completed
        (Utilities|FlowControl|Sequence
          (:then_0
            (CallFunction|Fire!))
          (:then_1
            (Utilities|FlowControl|Delay 1.0)
            (Utilities|FlowControl|Sequence
              (:then_0
                (goto _label_2 Reset))
              (:then_1
                (CallFunction|AutoFire)))))))
    (else
      (goto _label))))

(event Custom|Close_Click
  (Widget|RemovefromParent (stale OnClicked(TriggerBox) _returnvalue)))

(event Custom|Revert_Click
  (Game|SpawnActorfromClass "/Game/Placement/PlacementHub_BP.PlacementHub_BP_C" (Transformation|GetActorTransform) "Undefined" 0 0)
  (Actor|DestroyActor)
  (Widget|RemovefromParent (stale OnClicked(TriggerBox) _returnvalue))
  (bind _astdf_gamemode (Utilities|Casting|CastToTDF_Gamemode (Game|GetGameMode)))
  (Variables|/Game/User/TDF_Gamemode.TDF_Gamemode_C|SetPoints _astdf_gamemode (+ (Variables|/Game/User/TDF_Gamemode.TDF_Gamemode_C|GetPoints _astdf_gamemode) 700))
  (Variables|Default|SetUIActive false))

(event EventBeginPlay
  ;[1 1 1] Main Tower Loop
  (Utilities|FlowControl|Delay 0.1 :!label _label)
  (Utilities|FlowControl|Sequence
    (:then_0
      ;[1 1 1] Set Direction of Tower to aim at target
      (if (> (Utilities|Array|Length (Variables|Default|GetEnemyTargets)) 0)
        (Variables|Default|SetAutoShoot true)
        (bind _ascharacter (Utilities|Casting|CastToCharacter (Utilities|Array|Get(acopy) (Variables|Default|GetEnemyTargets))))
        (Transformation|SetWorldRotation (Variables|Default|GetTowerHead) (Math|Rotator|MakeRotator 0.0 0.0 (+ (.Yaw (Math|Rotator|BreakRotator (Math|Conversions|RotationFromXVector (Math|Vector|GetUnitDirection(Vector) (Transformation|GetWorldLocation (Variables|Default|GetTowerHead)) (Transformation|GetActorLocation _ascharacter))))) 1.8e+02)) false false)
        ;[1 1 1] First Target - Launch Firing Loop
        (Utilities|FlowControl|DoOnce false
          (:Completed
            (CallFunction|AutoFire)))
        (else
          (Variables|Default|SetAutoShoot false))))
    (:then_1
      (goto _label))))

(fn ConstructionScript)

(fn Fire!
  (Game|SpawnActorfromClass "/Game/Towers/GasTower/Upgrade/LongGasRound_BP.LongGasRound_BP_C" (Math|Transform|MakeTransform (Transformation|GetSocketLocation (Variables|Default|GetTowerHead) "Projectile") (Math|Rotator|MakeRotator 0.0 0.0 (+ (.Yaw (Math|Rotator|BreakRotator (Math|Conversions|RotationFromXVector (Variables|Default|GetShootDirection)))) 1.8e+02)) "0.500000,0.500000,0.500000") "Undefined" 0 0)
  (Audio|PlaySound2D "/Game/Audio/CannonBlast.CannonBlast" 1.0 1.0 0.0 0 0)
  (Components|Activation|SetActive (Variables|Default|GetBarrel2Blast) true false))