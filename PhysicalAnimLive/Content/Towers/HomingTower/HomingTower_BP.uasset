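; Tower-defense homing tower that launches homing projectiles at enemies in range and can be upgraded or sold.
; TriggerField overlaps maintain EnemyTargets using gamemode EnemyTags, while a Delay-based BeginPlay loop yaws HomingHead toward the first target.
; That loop starts AutoFire once, which repeatedly spawns projectiles homing on that target, about one per second.
; Clicking opens a UI that swaps the actor for HomingTowerUp_BP or PlacementHub_BP, adjusting gamemode Points.
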(event OnComponentBeginOverlap(TriggerField)
  (params (OverlappedComponent :type Primitive%20Component%20Object%20Reference) (OtherActor :type Actor%20Object%20Reference) (OtherComp :type Primitive%20Component%20Object%20Reference) (OtherBodyIndex :type Integer) (bFromSweep :type Boolean) (SweepResult :type Hit%20Result%20Structure%20%28by%20ref%29))
  ;[1 1 1] Track Incoming and Outgoing Targets
  (bind _aspawn (Utilities|Casting|CastToPawn OtherActor))
  (bind _astdf_gamemode (Utilities|Casting|CastToTDF_Gamemode (Game|GetGameMode)))
  (for _array_element (Variables|/Game/User/TDF_Gamemode.TDF_Gamemode_C|GetEnemyTags _astdf_gamemode)
    (if (Actor|ActorHasTag _aspawn _array_element)
      (Utilities|Array|Add (Variables|Default|GetEnemyTargets) OtherActor))))

(event OnComponentEndOverlap(TriggerField)
  (params (OverlappedComponent :type Primitive%20Component%20Object%20Reference) (OtherActor :type Actor%20Object%20Reference) (OtherComp :type Primitive%20Component%20Object%20Reference) (OtherBodyIndex :type Integer))
  ;[1 1 1] Track Incoming and Outgoing Targets
  (bind _aspawn (Utilities|Casting|CastToPawn OtherActor))
  (bind _astdf_gamemode (Utilities|Casting|CastToTDF_Gamemode (Game|GetGameMode)))
  (for _array_element (Variables|/Game/User/TDF_Gamemode.TDF_Gamemode_C|GetEnemyTags _astdf_gamemode)
    (if (Actor|ActorHasTag _aspawn _array_element)
      (Utilities|Array|RemoveItem (Variables|Default|GetEnemyTargets) OtherActor))))

(event OnClicked(Box)
  (params (TouchedComponent :type Primitive%20Component%20Object%20Reference) (ButtonPressed :type Key%20Structure))
  ;[1 1 1] Handles if the tower has been clicked on
  (if (not (Variables|Default|GetUIActive))
    (Variables|Default|SetUIActive true)
    (bind _returnvalue (UserInterface|CreateWidget "/Game/UI/HomingTowerUpgrade_UI.HomingTowerUpgrade_UI_C" (Game|GetPlayerController 0)))
    (UserInterface|Viewport|AddtoViewport _returnvalue 0)
    (EventDispatchers|AssignOnClicked (Variables|/Game/UI/HomingTowerUpgrade_UI.HomingTowerUpgrade_UI_C|GetUpgrade_BTN _returnvalue) (delegate Custom|UpgradeClicked))
    (EventDispatchers|BindEventtoOnClicked (Variables|/Game/UI/HomingTowerUpgrade_UI.HomingTowerUpgrade_UI_C|GetRevert_BTN _returnvalue) (delegate Custom|OnClickedRevert))
    (EventDispatchers|AssignOnClicked (Variables|/Game/UI/HomingTowerUpgrade_UI.HomingTowerUpgrade_UI_C|GetClose_BTN _returnvalue) (delegate Custom|Exit))))

(event Custom|AutoFire
  (bind _hominghead (Variables|Default|GetHomingHead))
  (bind _returnvalue (Transformation|GetWorldRotation _hominghead))
  (bind _returnvalue_2 (Math|Rotator|GetRotationXVector _returnvalue))
  (bind _returnvalue_3 (Math|Vector|Normalize _returnvalue_2))
  ;[1 1 1] Auto Firing Method
  (Utilities|FlowControl|Delay 0.1 :!label _label)
  (if (Variables|Default|GetAutoShoot)
    (Variables|Default|SetShoot%20Direction _returnvalue_3)
    (Variables|Default|SetSpawnLocation (+ _returnvalue_3 (Transformation|GetWorldLocation _hominghead)))
    (Utilities|FlowControl|DoOnce false :!label _label_2
      (:Completed
        (Utilities|FlowControl|Sequence
          (:then_0
            (CallFunction|FireHomingProjectile))
          (:then_1
            (Utilities|FlowControl|Delay 1.0)
            (Utilities|FlowControl|Sequence
              (:then_0
                (goto _label_2 Reset))
              (:then_1
                (CallFunction|AutoFire)))))))
    (else
      (goto _label))))

(event Custom|UpgradeClicked
  (bind _returnvalue (Transformation|GetActorLocation))
  ;[1 1 1] Handles if the tower has been clicked on
  (bind _astdf_gamemode (Utilities|Casting|CastToTDF_Gamemode (Game|GetGameMode)))
  (if (>= (Variables|/Game/User/TDF_Gamemode.TDF_Gamemode_C|GetPoints _astdf_gamemode) 800)
    (Audio|PlaySoundatLocation "/Game/Audio/BuySound.BuySound" _returnvalue "0, 0, 0" 1.0 1.0 0.0 0 0 0)
    (Game|SpawnActorfromClass "/Game/Towers/HomingTower/HomingTowerUpgrade/HomingTowerUp_BP.HomingTowerUp_BP_C" (Transformation|GetActorTransform) "Undefined" 0 0)
    (Variables|/Game/User/TDF_Gamemode.TDF_Gamemode_C|SetPoints _astdf_gamemode (- (Variables|/Game/User/TDF_Gamemode.TDF_Gamemode_C|GetPoints _astdf_gamemode) 800))
    (Widget|RemovefromParent (stale OnClicked(Box) _returnvalue))
    (Actor|DestroyActor)
    (Variables|Default|SetUIActive false)
    (else
      (Audio|PlaySoundatLocation "/Game/Audio/InsuffecientFunds.InsuffecientFunds" _returnvalue "0, 0, 0" 1.0 1.0 0.0 0 0 0))))

(event Custom|OnClickedRevert
  ;[1 1 1] Handles if the tower has been clicked on
  (Game|SpawnActorfromClass "/Game/Placement/PlacementHub_BP.PlacementHub_BP_C" (Transformation|GetActorTransform) "Undefined" 0 0)
  (Actor|DestroyActor)
  (Widget|RemovefromParent (stale OnClicked(Box) _returnvalue))
  (bind _astdf_gamemode (Utilities|Casting|CastToTDF_Gamemode (Game|GetGameMode)))
  (Variables|/Game/User/TDF_Gamemode.TDF_Gamemode_C|SetPoints _astdf_gamemode (+ (Variables|/Game/User/TDF_Gamemode.TDF_Gamemode_C|GetPoints _astdf_gamemode) 250))
  (Variables|Default|SetUIActive false))

(event Custom|Exit
  ;[1 1 1] Handles if the tower has been clicked on
  (Widget|RemovefromParent (stale OnClicked(Box) _returnvalue))
  (Variables|Default|SetUIActive false))

(event EventBeginPlay
  ;[1 1 1] Main Tower Loop
  (Utilities|FlowControl|Delay 0.1 :!label _label)
  (Utilities|FlowControl|Sequence
    (:then_0
      ;[1 1 1] Set Direction of Tower to aim at target
      (if (> (Utilities|Array|Length (Variables|Default|GetEnemyTargets)) 0)
        (Variables|Default|SetAutoShoot true)
        (bind _ascharacter (Utilities|Casting|CastToCharacter (Utilities|Array|Get(acopy) (Variables|Default|GetEnemyTargets))))
        (Transformation|SetWorldRotation (Variables|Default|GetHomingHead) (Math|Rotator|MakeRotator 0.0 0.0 (.Yaw (Math|Rotator|BreakRotator (Math|Conversions|RotationFromXVector (Math|Vector|GetUnitDirection(Vector) (Transformation|GetWorldLocation (Variables|Default|GetHomingHead)) (Transformation|GetActorLocation _ascharacter)))))) false false)
        ;[1 1 1] First Target - Launch FiringLoop
        (Utilities|FlowControl|DoOnce false
          (:Completed
            (CallFunction|AutoFire)))
        (else
          (Variables|Default|SetAutoShoot false))))
    (:then_1
      (goto _label))))

(fn ConstructionScript)

(fn FireHomingProjectile
  (bind _hominghead (Variables|Default|GetHomingHead))
  (bind _returnvalue (Transformation|GetSocketLocation _hominghead "Projectile"))
  (Components|Activation|SetActive (Variables|Default|GetParticleSystem) true true)
  (Audio|SpawnSoundatLocation "/Game/Towers/HomingTower/Missle_Launch.Missle_Launch" _returnvalue "0, 0, 0" 0.1 1.0 1.5 0 0)
  (bind _returnvalue_2 (Game|SpawnActorfromClass "/Game/Towers/HomingTower/HomingProjectle_BP.HomingProjectle_BP_C" (Math|Transform|MakeTransform _returnvalue (Math|Rotator|MakeRotator 0.0 0.0 (+ (.Yaw (Math|Rotator|BreakRotator (Math|Conversions|RotationFromXVector (Variables|Default|GetShoot%20Direction)))) 0.0)) "0.100000,0.100000,0.100000") "Undefined" 0 0))
  (bind _asai_character (Utilities|Casting|CastToAI_Character (Utilities|Array|Get(acopy) (Variables|Default|GetEnemyTargets))))
  (Variables|/Script/Engine.ProjectileMovementComponent|SetHomingTargetComponent (Variables|/Game/Towers/HomingTower/HomingProjectle_BP.HomingProjectle_BP_C|GetProjectileMovement _returnvalue_2) (Variables|/Script/Engine.Actor|GetRootComponent _asai_character)))