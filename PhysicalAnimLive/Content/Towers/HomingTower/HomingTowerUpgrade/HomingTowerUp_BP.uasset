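; Upgraded homing missile tower for a tower defense game, firing four-missile salvos at enemies within its trigger field.
; Overlap events maintain EnemyTargets using gamemode tags, while a looping BeginPlay timer yaws the head toward the first target.
; A self-restarting AutoFire loop launches homing projectiles from four sockets with effects and sound.
; Clicking the box opens a revert UI that swaps the tower for a placement hub and refunds points.
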(event OnClicked(Box)
  (params (TouchedComponent :type Primitive%20Component%20Object%20Reference) (ButtonPressed :type Key%20Structure))
  (bind _returnvalue (UserInterface|CreateWidget "/Game/UI/Revert_UI.Revert_UI_C" (Game|GetPlayerController 0)))
  (UserInterface|Viewport|AddtoViewport _returnvalue 0)
  (EventDispatchers|BindEventtoOnClicked (Variables|/Game/UI/Revert_UI.Revert_UI_C|GetRevert_BTN _returnvalue) (delegate Custom|OnClickedRevert)))

(event OnComponentEndOverlap(TriggerField)
  (params (OverlappedComponent :type Primitive%20Component%20Object%20Reference) (OtherActor :type Actor%20Object%20Reference) (OtherComp :type Primitive%20Component%20Object%20Reference) (OtherBodyIndex :type Integer))
  ;[1 1 1] Track Incoming and Outgoing Targets
  (bind _aspawn (Utilities|Casting|CastToPawn OtherActor))
  (bind _astdf_gamemode (Utilities|Casting|CastToTDF_Gamemode (Game|GetGameMode)))
  (for _array_element (Variables|/Game/User/TDF_Gamemode.TDF_Gamemode_C|GetEnemyTags _astdf_gamemode)
    (if (Actor|ActorHasTag _aspawn _array_element)
      (Utilities|Array|RemoveItem (Variables|Default|GetEnemyTargets) OtherActor))))

(event OnComponentBeginOverlap(TriggerField)
  (params (OverlappedComponent :type Primitive%20Component%20Object%20Reference) (OtherActor :type Actor%20Object%20Reference) (OtherComp :type Primitive%20Component%20Object%20Reference) (OtherBodyIndex :type Integer) (bFromSweep :type Boolean) (SweepResult :type Hit%20Result%20Structure%20%28by%20ref%29))
  ;[1 1 1] Track Incoming and Outgoing Targets
  (bind _aspawn (Utilities|Casting|CastToPawn OtherActor))
  (bind _astdf_gamemode (Utilities|Casting|CastToTDF_Gamemode (Game|GetGameMode)))
  (for _array_element (Variables|/Game/User/TDF_Gamemode.TDF_Gamemode_C|GetEnemyTags _astdf_gamemode)
    (if (Actor|ActorHasTag _aspawn _array_element)
      (Utilities|Array|Add (Variables|Default|GetEnemyTargets) OtherActor))))

(event Custom|AutoFire
  (bind _hominghead (Variables|Default|GetHomingHead))
  (bind _returnvalue (Transformation|GetWorldRotation _hominghead))
  (bind _returnvalue_2 (Math|Rotator|GetRotationXVector _returnvalue))
  (bind _returnvalue_3 (Math|Vector|Normalize _returnvalue_2))
  ;[1 1 1] Auto Firing Method
  (Utilities|FlowControl|Delay 0.8 :!label _label)
  (if (Variables|Default|GetAutoShoot)
    (Variables|Default|SetShoot%20Direction _returnvalue_3)
    (Variables|Default|SetSpawnLocation (+ _returnvalue_3 (Transformation|GetWorldLocation _hominghead)))
    (Utilities|FlowControl|DoOnce false :!label _label_2
      (:Completed
        (Utilities|FlowControl|Sequence
          (:then_0
            (CallFunction|FireHomingProjectile))
          (:then_1
            (Utilities|FlowControl|Delay 1.0)
            (Utilities|FlowControl|Sequence
              (:then_0
                (goto _label_2 Reset))
              (:then_1
                (CallFunction|AutoFire)))))))
    (else
      (goto _label))))

(event Custom|OnClickedRevert
  (Game|SpawnActorfromClass "/Game/Placement/PlacementHub_BP.PlacementHub_BP_C" (Transformation|GetActorTransform) "Undefined" 0 0)
  (Actor|DestroyActor)
  (Widget|RemovefromParent (stale OnClicked(Box) _returnvalue))
  (bind _astdf_gamemode (Utilities|Casting|CastToTDF_Gamemode (Game|GetGameMode)))
  (Variables|/Game/User/TDF_Gamemode.TDF_Gamemode_C|SetPoints _astdf_gamemode (+ (Variables|/Game/User/TDF_Gamemode.TDF_Gamemode_C|GetPoints _astdf_gamemode) 650)))

(event EventBeginPlay
  ;[1 1 1] Main Tower Loop
  (Utilities|FlowControl|Delay 0.1 :!label _label)
  (Utilities|FlowControl|Sequence
    (:then_0
      ;[1 1 1] Set Direction of Tower to aim at target
      (if (> (Utilities|Array|Length (Variables|Default|GetEnemyTargets)) 0)
        (Variables|Default|SetAutoShoot true)
        (bind _ascharacter (Utilities|Casting|CastToCharacter (Utilities|Array|Get(acopy) (Variables|Default|GetEnemyTargets))))
        (Transformation|SetWorldRotation (Variables|Default|GetHomingHead) (Math|Rotator|MakeRotator 0.0 0.0 (+ (.Yaw (Math|Rotator|BreakRotator (Math|Conversions|RotationFromXVector (Math|Vector|GetUnitDirection(Vector) (Transformation|GetWorldLocation (Variables|Default|GetHomingBase)) (Transformation|GetActorLocation _ascharacter))))) -95.0)) false false)
        ;[1 1 1] First Target - Launch FiringLoop
        (Utilities|FlowControl|DoOnce false
          (:Completed
            (CallFunction|AutoFire)))
        (else
          (Variables|Default|SetAutoShoot false))))
    (:then_1
      (goto _label))))

(fn ConstructionScript)

(fn FireHomingProjectile
  (Utilities|FlowControl|Sequence
    (:then_0
      (|FireFirstProjectile))
    (:then_1
      (|FireSecondProjectile))
    (:then_2
      (|FireThirdProjectile))
    (:then_3
      (|FireFourthProjectile))))