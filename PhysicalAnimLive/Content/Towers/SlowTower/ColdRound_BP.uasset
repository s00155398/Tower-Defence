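; Cold projectile for the slow tower that damages and slows the enemy it hits, then destroys itself.
; On collision overlap it matches the actor's tags against the game mode's EnemyTags, then plays freeze particles and sound at the enemy.
; It subtracts Damage directly from the enemy's Health, halved for Invigored enemies, and calls SlowCharacter.
; Rounds that hit nothing expire after a short fixed lifetime.
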(event OnComponentBeginOverlap(CollisionComponent)
  (params (OverlappedComponent :type Primitive%20Component%20Object%20Reference) (OtherActor :type Actor%20Object%20Reference) (OtherComp :type Primitive%20Component%20Object%20Reference) (OtherBodyIndex :type Integer) (bFromSweep :type Boolean) (SweepResult :type Hit%20Result%20Structure%20%28by%20ref%29))
  (bind _astdf_gamemode (Utilities|Casting|CastToTDF_Gamemode (Game|GetGameMode)))
  (for _array_element (Variables|/Game/User/TDF_Gamemode.TDF_Gamemode_C|GetEnemyTags _astdf_gamemode)
    (if (Actor|ActorHasTag OtherActor _array_element)
      (bind _asbase_enemy_class_bp (Utilities|Casting|CastToBaseEnemyClass_BP OtherActor))
      (Effects|SpawnEmitteratLocation "/Game/Materials/Effects/P_ColdHit.P_ColdHit" (Transformation|GetActorLocation _asbase_enemy_class_bp))
      (Audio|SpawnSoundatLocation "/Game/Audio/Fast_Freezing_ice_SOUND_Effect.Fast_Freezing_ice_SOUND_Effect" (Transformation|GetActorLocation _asbase_enemy_class_bp) "0, 0, 0" 0.15 1.0 2.0 0 0)
      (if (Variables|/Game/AI/Enemies/BaseEnemyClass_BP.BaseEnemyClass_BP_C|GetInvigored _asbase_enemy_class_bp)
        (Variables|/Game/AI/Enemies/BaseEnemyClass_BP.BaseEnemyClass_BP_C|SetHealth _asbase_enemy_class_bp (- (Variables|/Game/AI/Enemies/BaseEnemyClass_BP.BaseEnemyClass_BP_C|GetHealth _asbase_enemy_class_bp) (/ (Variables|Default|GetDamage) 2.0)))
        (else
          (Variables|/Game/AI/Enemies/BaseEnemyClass_BP.BaseEnemyClass_BP_C|SetHealth _asbase_enemy_class_bp (- (Variables|/Game/AI/Enemies/BaseEnemyClass_BP.BaseEnemyClass_BP_C|GetHealth _asbase_enemy_class_bp) (Variables|Default|GetDamage)))))
      (Default|SlowCharacter _asbase_enemy_class_bp)
      (Actor|DestroyActor))))

(event EventBeginPlay
  (Utilities|FlowControl|Delay 5.0)
  (Actor|DestroyActor))

(fn ConstructionScript)