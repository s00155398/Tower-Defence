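; Upgraded cold tower projectile that slows enemies in an area when it hits one, and destroys itself after five seconds otherwise.
; Hitting an actor with a gamemode enemy tag spawns a freeze effect and sound, then briefly enables overlap events on an explosion radius before destroying the round.
; Actors overlapping that radius are collected, and each tagged enemy among them has SlowCharacter called on it.
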(event OnComponentBeginOverlap(ExplosionRadius)
  (params (OverlappedComponent :type Primitive%20Component%20Object%20Reference) (OtherActor :type Actor%20Object%20Reference) (OtherComp :type Primitive%20Component%20Object%20Reference) (OtherBodyIndex :type Integer) (bFromSweep :type Boolean) (SweepResult :type Hit%20Result%20Structure%20%28by%20ref%29))
  (Utilities|Array|Add (Variables|Default|GetEnemiesHit) OtherActor)
  (for _array_element (Variables|Default|GetEnemiesHit)
    (bind _astdf_gamemode (Utilities|Casting|CastToTDF_Gamemode (Game|GetGameMode)))
    (for _array_element_2 (Variables|/Game/User/TDF_Gamemode.TDF_Gamemode_C|GetEnemyTags _astdf_gamemode)
      (if (Actor|ActorHasTag _array_element _array_element_2)
        (bind _asbase_enemy_class_bp (Utilities|Casting|CastToBaseEnemyClass_BP _array_element))
        (Default|SlowCharacter _asbase_enemy_class_bp)))))

(event OnComponentBeginOverlap(CollisionComponent)
  (params (OverlappedComponent :type Primitive%20Component%20Object%20Reference) (OtherActor :type Actor%20Object%20Reference) (OtherComp :type Primitive%20Component%20Object%20Reference) (OtherBodyIndex :type Integer) (bFromSweep :type Boolean) (SweepResult :type Hit%20Result%20Structure%20%28by%20ref%29))
  (bind _returnvalue (Transformation|GetActorLocation OtherActor))
  (bind _astdf_gamemode (Utilities|Casting|CastToTDF_Gamemode (Game|GetGameMode)))
  (for _array_element (Variables|/Game/User/TDF_Gamemode.TDF_Gamemode_C|GetEnemyTags _astdf_gamemode)
    (if (Actor|ActorHasTag OtherActor _array_element)
      (Effects|SpawnEmitteratLocation "/Game/Materials/Effects/P_ColdHit.P_ColdHit" _returnvalue "0, 0, 0" "3.000000,3.000000,3.000000")
      (Audio|SpawnSoundatLocation "/Game/Audio/Fast_Freezing_ice_SOUND_Effect.Fast_Freezing_ice_SOUND_Effect" _returnvalue "0, 0, 0" 0.15 1.0 2.0 0 0)
      (Variables|/Script/Engine.PrimitiveComponent|SetbGenerateOverlapEvents (Variables|Default|GetExplosionRadius) true)
      (Utilities|FlowControl|Delay 0.01)
      (Actor|DestroyActor))))

(event EventBeginPlay
  (Utilities|FlowControl|Delay 5.0)
  (Actor|DestroyActor))

(fn ConstructionScript)