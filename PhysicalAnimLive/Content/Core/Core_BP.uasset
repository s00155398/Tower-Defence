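; Core actor that acts as a damageable objective, losing health when enemies reach it.
; Overlaps on its DamageZone check the actor against the enemy tags from TDF_Gamemode.
; A match spawns an impact Niagara effect, destroys the enemy and subtracts a fixed amount of health.
; When health runs out, it reloads the current level.
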(event OnComponentBeginOverlap(DamageZone)
  (params (OverlappedComponent :type Primitive%20Component%20Object%20Reference) (OtherActor :type Actor%20Object%20Reference) (OtherComp :type Primitive%20Component%20Object%20Reference) (OtherBodyIndex :type Integer) (bFromSweep :type Boolean) (SweepResult :type Hit%20Result%20Structure%20%28by%20ref%29))
  (bind _astdf_gamemode (Utilities|Casting|CastToTDF_Gamemode (Game|GetGameMode)))
  (for _array_element (Variables|/Game/User/TDF_Gamemode.TDF_Gamemode_C|GetEnemyTags _astdf_gamemode)
    (if (Actor|ActorHasTag OtherActor _array_element)
      (Niagara|SpawnSystematLocation "/Game/Core/Impact_NS.Impact_NS" (Transformation|GetActorLocation OtherActor))
      (Actor|DestroyActor OtherActor)
      (Variables|Default|SetHealth (- (Variables|Default|GetHealth) 25.0))
      (if (<= (Variables|Default|GetHealth) 0.0)
        (bind _returnvalue (Game|GetCurrentLevelName true))
        (Game|OpenLevel(byName) (Utilities|String|StringToName _returnvalue))))))

(event EventBeginPlay)

(event Collision|EventActorBeginOverlap
  (params (OtherActor :type Actor%20Object%20Reference)))

(event EventTick
  (params (DeltaSeconds :type Float%20%28single-precision%29)))

(fn ConstructionScript)